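; CollectableBP is a pickup actor for a collect-to-win game, collected when the first-person character overlaps its BoxCollision.
; On overlap it decrements CollectablesLeft on BP_FirstPersonGameMode, adds a new CollectableWidgetBP to the viewport, then destroys itself.
; End overlap disables player input on the actor, a leftover of an input-based collection approach whose EnableInput node is unconnected.
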(event OnComponentBeginOverlap(BoxCollision)
  (params (OverlappedComponent :type Primitive%20Component%20Object%20Reference) (OtherActor :type Actor%20Object%20Reference) (OtherComp :type Primitive%20Component%20Object%20Reference) (OtherBodyIndex :type Integer) (bFromSweep :type Boolean) (SweepResult :type Hit%20Result%20Structure%20%28by%20ref%29))
  (Utilities|Casting|CastToBP_FirstPersonCharacter OtherActor)
  (bind _asbp_first_person_game_mode (Utilities|Casting|CastToBP_FirstPersonGameMode (Game|GetGameMode)))
  (bind _result (Math|Integer|DecrementInt (Variables|/Game/FirstPerson/Blueprints/BP_FirstPersonGameMode.BP_FirstPersonGameMode_C|GetCollectablesLeft _asbp_first_person_game_mode))
    (:%20%20
      (Variables|/Game/FirstPerson/Blueprints/BP_FirstPersonGameMode.BP_FirstPersonGameMode_C|SetCollectablesLeft _asbp_first_person_game_mode _result)
      (bind _returnvalue (UserInterface|CreateWidget "/Game/CollectXtoWin/CollectableWidgetBP.CollectableWidgetBP_C"))
      (UserInterface|Viewport|AddtoViewport _returnvalue 0)
      (Actor|DestroyActor))))

(event OnComponentEndOverlap(BoxCollision)
  (params (OverlappedComponent :type Primitive%20Component%20Object%20Reference) (OtherActor :type Actor%20Object%20Reference) (OtherComp :type Primitive%20Component%20Object%20Reference) (OtherBodyIndex :type Integer))
  ;[1 1 1] collecting with input. needs begin overlap and cast to bp as below
  (Utilities|Casting|CastToBP_FirstPersonCharacter OtherActor)
  (Input|DisableInput (Game|GetPlayerController 0)))

(fn ConstructionScript)